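; Turret actor that turns to face the player and fires a limited series of bullets.
; After an initial delay it activates, aiming at player character 0 every tick with a -90 pitch offset.
; A delay loop spawns Bullet_BP at ProjectileSpawnPoint once per second until the index passes MaxBullets.
; The construction script sets delay and bullet limit from value variables; a VariableDatabase_BP lookup is left unconnected.
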(event EventTick
  (params (DeltaSeconds :type Float%20%28single-precision%29))
  (if (Variables|Default|GetIsActive)
    (CallFunction|SetRotation)))

(event EventBeginPlay
  (Utilities|FlowControl|Delay (Variables|Default|GetInitialDelay))
  (Variables|Default|SetIsActive true)
  (if (<= (Variables|Default|GetIndex) (Variables|Default|GetMaxBullets)) :!label _label
    (Utilities|FlowControl|Delay 1.0)
    (CallFunction|FireBullet)
    (Variables|Default|SetIndex (+ (Variables|Default|GetIndex) 1))
    (goto _label)))

(fn ConstructionScript
  (Variables|Default|SetInitialDelay (Variables|Default|GetInitialDelayValue))
  (Variables|Default|SetMaxBullets (Variables|Default|GetMaxBulletsValue)))

(fn FireBullet
  (Game|SpawnActorfromClass "/Game/Blueprints/Bullet_BP.Bullet_BP_C" (Transformation|GetWorldTransform (Variables|Default|GetProjectile%20Spawn%20Point)) "Undefined" 0 0))

(fn SetRotation
  (bind _returnvalue (Game|GetPlayerCharacter 0))
  (bind _returnvalue_2 (Transformation|GetActorLocation))
  (bind _returnvalue_3 (Transformation|GetActorLocation _returnvalue))
  (bind _returnvalue_4 (Math|Rotator|FindLookatRotation _returnvalue_2 _returnvalue_3))
  (Transformation|SetActorRotation (Math|Rotator|MakeRotator (.roll _returnvalue_4) (+ (.pitch _returnvalue_4) -9e+01) (.yaw _returnvalue_4))))