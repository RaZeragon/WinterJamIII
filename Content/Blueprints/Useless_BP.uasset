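; Useless_BP is a Blueprint with a camera and basic health tracking; its wider role is not evident.
; Pressing the right mouse button snaps the Camera to Arrow2's relative location, with no handler to move it back.
; CalculateHealth adds a delta to Health, then CalculateDead sets IsDead when Health is zero or below.
; The event graph never calls the health functions and holds an unconnected SetRelativeLocation node.
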(event Input|MouseEvents|RightMouseButton
  (params (Key :type Key%20Structure)))

(event Input|MouseEvents|RightMouseButton
  (params (Key :type Key%20Structure))
  (:Pressed
    (Transformation|SetRelativeLocation (Variables|Default|GetCamera) (Variables|/Script/Engine.SceneComponent|GetRelativeLocation (Variables|Default|GetArrow2)) false false)))

(fn ConstructionScript)

(fn CalculateDead
  ;[1 1 1] If health goes beneath 0, set IsDead to true
  (if (<= (Variables|Default|GetHealth) 0.0)
    (Variables|Default|SetIsDead true)
    (else
      (Variables|Default|SetIsDead false))))

(fn CalculateHealth
  (params (Delta :type Float%20%28single-precision%29))
  (Variables|Default|SetHealth (+ Delta (Variables|Default|GetHealth)))
  (CallFunction|CalculateDead))