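; BigBoy_BP is a controllable shooter pawn with mouse look, health and a right-click toggle between first and third person camera positions.
; Left click spawns GunBullet_BP at the gun, then steps the pawn backward against the aim direction as decaying, delayed recoil.
; AffectHealth applies changes through CalculateHealth and CalculateDead, destroying the actor at zero.
; FireGunBullet duplicates firing without delay but is uncalled here; gun-aiming logic is disconnected.
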(event EventAffectHealth
  (params (Delta :type Float%20%28single-precision%29))
  (CallFunction|CalculateHealth Delta)
  (Development|PrintString (Utilities|String|ToString(Float) (Variables|Default|GetHealth)))
  (if (Variables|Default|GetIsDead)
    (Actor|DestroyActor)))

(event Input|AxisEvents|InputAxisLookRight
  (params (AxisValue :type Float%20%28single-precision%29))
  ;[1 1 1] Mouse controls
  (Pawn|Input|AddControllerYawInput AxisValue))

(event Input|AxisEvents|InputAxisLookUp
  (params (AxisValue :type Float%20%28single-precision%29))
  ;[1 1 1] Mouse controls
  (Pawn|Input|AddControllerPitchInput AxisValue))

(event Input|MouseEvents|RightMouseButton
  (params (Key :type Key%20Structure))
  (bind _camera (Variables|Default|GetCamera))
  ;[1 1 1] Toggle between first and third person view
  (:Pressed
    (Utilities|FlowControl|FlipFlop
      (:A
        (Transformation|SetRelativeLocation _camera (Variables|/Script/Engine.SceneComponent|GetRelativeLocation (Variables|Default|GetThird%20Person)) false false))
      (:B
        (Transformation|SetRelativeLocation _camera (Variables|/Script/Engine.SceneComponent|GetRelativeLocation (Variables|Default|GetFirst%20Person)) false false)))))

(event Input|MouseEvents|LeftMouseButton
  (params (Key :type Key%20Structure))
  (bind _returnvalue (Pawn|GetControlRotation :!class /Script/Engine.Pawn))
  (:Pressed
    (Game|SpawnActorfromClass "/Game/Blueprints/GunBullet_BP.GunBullet_BP_C" (Transformation|GetWorldTransform (Variables|Default|GetGun)) "Undefined" 0 0)
    (Variables|Default|SetVelocity 1e+01)
    (while (> (Variables|Default|GetVelocity) 0.0)
      (Variables|Default|SetVelocity (- (Variables|Default|GetVelocity) 0.5))
      (Utilities|FlowControl|Delay 0.3)
      (Transformation|SetActorLocation (+ (Transformation|GetActorLocation) (* (Class|KismetMathLibrary|CreateVectorfromYawPitch (.yaw _returnvalue) (.pitch _returnvalue) 1.0) (* (Variables|Default|GetVelocity) -1.0))) false false))))

(fn ConstructionScript)

(fn FireGunBullet
  (bind _returnvalue (Pawn|GetControlRotation :!class /Script/Engine.Pawn))
  (Game|SpawnActorfromClass "/Game/Blueprints/GunBullet_BP.GunBullet_BP_C" (Transformation|GetWorldTransform (Variables|Default|GetGun)) "Undefined" 0 0)
  (Variables|Default|SetVelocity 1e+01)
  (while (> (Variables|Default|GetVelocity) 0.0)
    (Variables|Default|SetVelocity (- (Variables|Default|GetVelocity) 0.5))
    (Transformation|SetActorLocation (+ (Transformation|GetActorLocation) (* (Class|KismetMathLibrary|CreateVectorfromYawPitch (.yaw _returnvalue) (.pitch _returnvalue) 1.0) (* (Variables|Default|GetVelocity) -1.0))) false false)))

(fn CalculateHealth
  (params (Delta :type Float%20%28single-precision%29))
  ;[1 1 1] Calculating health by adding the changes to health
  (Variables|Default|SetHealth (+ Delta (Variables|Default|GetHealth)))
  (CallFunction|CalculateDead))

(fn CalculateDead
  ;[1 1 1] If health <= 0, set IsDead to true
  (if (<= (Variables|Default|GetHealth) 0.0)
    (Variables|Default|SetIsDead true)
    (else
      (Variables|Default|SetIsDead false))))