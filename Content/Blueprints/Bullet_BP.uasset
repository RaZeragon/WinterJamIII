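; Bullet projectile actor that deals damage on overlap and bounces until it reaches a bounce limit.
; Overlapping an IDamageable actor sends it the Damage value through AffectHealthMessage, then destroys the bullet.
; ProjectileMovement's bounce event increments a counter and destroys the bullet at a hardcoded count.
; An unfinished, disconnected branch would adjust rotation based on Wall and axis tags but never runs.
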(event OnProjectileBounce(ProjectileMovement)
  (params (ImpactResult :type Hit%20Result%20Structure%20%28by%20ref%29) (ImpactVelocity :type Vector%20%28by%20ref%29 :default "0, 0, 0"))
  (bind _result (Math|Integer|IncrementInt (Variables|Default|GetnumBounces))
    (:%20%20
      (bind _output_get (Variables|Default|SetmaxBounces (== _result 15)))
      (if _output_get
        (Actor|DestroyActor)))))

(event Collision|EventActorBeginOverlap
  (params (OtherActor :type Actor%20Object%20Reference))
  (if (Utilities|DoesObjectImplementInterface OtherActor "/Game/Blueprints/iDamageable.iDamageable_C")
    (Class|IDamageable|AffectHealth(Message) OtherActor (Variables|Default|GetDamage))
    (Actor|DestroyActor)))

(fn ConstructionScript)